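; Spline-based road actor that builds a deformed road mesh along an editable spline in the construction script.
; Each spline segment gets a SplineMeshComponent matching point positions, tangents and Y/Z scale.
; All segments share one dynamic material instance fed by exposed falloff, opacity, normal, dirt, tiling and noise settings.
; Custom primitive data flags the first and last segments with opposite signs, likely for end fading.
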(fn `UserConstructionScript`
  (locals (RoadMaterial :type "MaterialInterface Object Reference" :default "/Script/Engine.Material'/Game/Landscape/Road/M_Road.M_Road'") (RoadMaterialInstance :type "MaterialInstanceDynamic Object Reference" :default null))
  (bind _roadmaterialinstance (`local.RoadMaterialInstance`))
  (bind _spline (`self.Spline`))
  (bind _returnvalue (`KismetMaterialLibrary.CreateDynamicMaterialInstance` (`local.RoadMaterial`)))
  (set `local.RoadMaterialInstance` _returnvalue)
  (for _index (range (+ (- (`SplineComponent.GetNumberOfSplinePoints` (`self.Spline`)) 2) 1))
    (bind _returnvalue_2 (`AddComponent|NODE_AddSplineMeshComponent-0`))
    (`SplineMeshComponent.SetForwardAxis` _returnvalue_2 "X" true)
    (bind _returnvalue_3 (+ _index 1))
    (`SplineMeshComponent.SetStartAndEnd` _returnvalue_2 (`SplineComponent.GetLocationAtSplinePoint` _spline _index "Local") (`SplineComponent.GetTangentAtSplinePoint` _spline _index "Local") (`SplineComponent.GetLocationAtSplinePoint` _spline _returnvalue_3 "Local") (`SplineComponent.GetTangentAtSplinePoint` _spline _returnvalue_3 "Local") true)
    (bind (_returnvalue_x _returnvalue_y _returnvalue_z) (`KismetMathLibrary.BreakVector` (`SplineComponent.GetScaleAtSplinePoint` _spline _index)))
    (`SplineMeshComponent.SetStartScale` _returnvalue_2 (`KismetMathLibrary.MakeVector2D` _returnvalue_y _returnvalue_z) true)
    (bind (_returnvalue_x_2 _returnvalue_y_2 _returnvalue_z_2) (`KismetMathLibrary.BreakVector` (`SplineComponent.GetScaleAtSplinePoint` _spline _returnvalue_3)))
    (`SplineMeshComponent.SetEndScale` _returnvalue_2 (`KismetMathLibrary.MakeVector2D` _returnvalue_y_2 _returnvalue_z_2) true)
    (`PrimitiveComponent.SetMaterial` _returnvalue_2 0 (`local.RoadMaterialInstance`))
    (if (== _index 0)
      (`PrimitiveComponent.SetCustomPrimitiveDataFloat` _returnvalue_2 0 1.0)
      (elif (== _index (- (`SplineComponent.GetNumberOfSplinePoints` (`self.Spline`)) 2))
        (`PrimitiveComponent.SetCustomPrimitiveDataFloat` _returnvalue_2 0 -1.0))))
  (`MaterialInstanceDynamic.SetScalarParameterValue` _roadmaterialinstance "RoadFalloffOffset" (`self.RoadFalloffOffset`))
  (`MaterialInstanceDynamic.SetScalarParameterValue` _roadmaterialinstance "RoadFalloffHardness" (`self.RoadFalloffHardness`))
  (`MaterialInstanceDynamic.SetScalarParameterValue` _roadmaterialinstance "RoadOpacityContrast" (`self.RoadOpacityContrast`))
  (`MaterialInstanceDynamic.SetScalarParameterValue` _roadmaterialinstance "NormalFlatness" (`self.RoadNormalFlatness`))
  (`MaterialInstanceDynamic.SetScalarParameterValue` _roadmaterialinstance "DirtOffset" (`self.DirtOffset`))
  (`MaterialInstanceDynamic.SetScalarParameterValue` _roadmaterialinstance "DirtContrast" (`self.DirtContrast`))
  (`MaterialInstanceDynamic.SetScalarParameterValue` _roadmaterialinstance "Tiling X" (`self.TilingX`))
  (`MaterialInstanceDynamic.SetScalarParameterValue` _roadmaterialinstance "Tiling Y" (`self.TilingY`))
  (`MaterialInstanceDynamic.SetScalarParameterValue` _roadmaterialinstance "NoiseInfluence" (`self.NoiseInfluence`))
  (`MaterialInstanceDynamic.SetScalarParameterValue` _roadmaterialinstance "DirtColour" (`self.DirtColour`))
  (`MaterialInstanceDynamic.SetScalarParameterValue` _roadmaterialinstance "RoadEndFalloffHardness" (`self.RoadEndFalloffHardness`)))